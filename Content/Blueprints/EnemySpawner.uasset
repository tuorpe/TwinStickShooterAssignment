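; EnemySpawner spawns AI-controlled EnemyCharacter pawns inside a box volume, up to an adjustable population limit.
; SpawnEnemy counts every EnemyCharacter in the world and, below MaxEnemies, spawns one at a random point within SpawnVolume.
; IncrementEnemyLimit raises that cap by one.
; Neither event is called within the Blueprint, which has no active BeginPlay or Tick logic.
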(event `SpawnEnemy`
  (bind _spawnvolume (`self.SpawnVolume`))
  (bind _outactors (`GameplayStatics.GetAllActorsOfClass` "/Game/Blueprints/EnemyCharacter.EnemyCharacter_C"))
  (if (< (`KismetArrayLibrary.Array_Length` _outactors) (`self.MaxEnemies`))
    (`AIBlueprintHelperLibrary.SpawnAIFromClass` "/Game/Blueprints/EnemyCharacter.EnemyCharacter_C" null (`KismetMathLibrary.RandomPointInBoundingBox` (`SceneComponent.K2_GetComponentLocation` _spawnvolume) (`BoxComponent.GetScaledBoxExtent` _spawnvolume)) (struct) false null)))

(event `IncrementEnemyLimit`
  (bind _result (`/Engine/EditorBlueprintResources/StandardMacros.IncrementInt` (`self.MaxEnemies`))
    (:`  `
      (set `self.MaxEnemies` _result))))

(fn `UserConstructionScript`)