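; MainMenuHero is the main menu's display hero, shown armed and slowly rotating in a twin-stick game.
; On BeginPlay it spawns a weapon on the mesh's GunSocket, attaches gun smoke at the projectile spawn point and shows the mouse cursor.
; It also saves its own transform as the TwinStickMode game mode's player spawn transform.
; Tick turns the SelfieStick by a small fixed step each frame, independent of delta time.
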(event `self.ReceiveBeginPlay`
  (bind _mesh (`self.Mesh`))
  ;[1 1 1] Gun spawner & gun smoke particle effect start
  (`|ExecutionSequence`
    (:`then_0`
      (bind _returnvalue (`|SpawnActorFromClass` "/Game/Blueprints/Weapon.Weapon_C" (`SceneComponent.K2_GetComponentToWorld` _mesh) "Undefined" "MultiplyWithRoot" null null))
      (bind _output_get (set `self.Weapon` _returnvalue))
      (`self.K2_AttachToComponent` _output_get _mesh "GunSocket" "SnapToTarget" "KeepRelative" "KeepRelative" true)
      (`GameplayStatics.SpawnEmitterAttached` "/Game/StarterContent/Particles/GunSmoke.GunSmoke" (`/Game/Blueprints/Weapon.ProjectileSpawnPoint` (`self.Weapon`)) "None" (10.0 0.0 0.0))
      ;[1 1 1] Show mouse cursor in main menu
      (set `PlayerController.bShowMouseCursor` true (`GameplayStatics.GetPlayerController` 0)))
    (:`then_1`
      (bind _astwin_stick_mode (cast `/Game/Blueprints/TwinStickMode` (`GameplayStatics.GetGameMode`)))
      (bind _output_get_2 (set `self.GameMode` _astwin_stick_mode))
      (set `/Game/Blueprints/TwinStickMode.PlayerSpawnTransform` (`self.GetTransform`) _output_get_2))))

(event `self.ReceiveTick`
  (params (DeltaSeconds :type "Float (single-precision)"))
  (bind _selfiestick (`self.SelfieStick`))
  ;[1 1 1] Hero slow rotate
  (`GameplayStatics.GetActorOfClass` "MainMenuHero_C")
  (`SceneComponent.K2_SetWorldRotation` _selfiestick (`KismetMathLibrary.NormalizedDeltaRotator` (`SpringArmComponent.GetTargetRotation` _selfiestick) (struct :`Yaw` 0.1)) false false))

(fn `UserConstructionScript`)